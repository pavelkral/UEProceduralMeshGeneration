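; AI character that chases the player on sight and plays a left-hook attack montage on reaching them.
; PawnSensing sighting sets a movement flag and runs AIMoveTo toward the player character.
; Arrival clears the flag, so Tick halts movement, and a second flag blocks montage replays until a delay matching its length ends.
; A failed move stops the montage and resets both flags.
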(event `self.ReceiveTick`
  (params (DeltaSeconds :type "Float (single-precision)"))
  (if (not (`self.camMove`))
    ;[1 1 1] Comment
    (`MovementComponent.StopMovementImmediately` (`self.CharacterMovement`))))

(event `self.PawnSensing.OnSeePawn`
  (params (Pawn :type "Pawn Object Reference"))
  (set `self.camMove` true)
  (`self.followPawn`)
  (`KismetSystemLibrary.PrintString` "Visible"))

(event `followPawn`
  (if (`self.camMove`)
    (`|AIMoveTo` self (0.0 0.0 0.0) (`GameplayStatics.GetPlayerCharacter` 0) 70.0
      (:`OnSuccess`
        (`KismetSystemLibrary.PrintString` "Rached")
        (set `self.camMove` false)
        (if (`self.bCanPlay`)
          (set `self.bCanPlay` false)
          (bind _returnvalue (`self.PlayAnimMontage` "/Game/atNinjaLeftHook_Montage.atNinjaLeftHook_Montage"))
          (`KismetSystemLibrary.Delay` _returnvalue)
          (`KismetSystemLibrary.PrintString` "Plyaed")
          (set `self.bCanPlay` true)))
      (:`OnFail`
        (`self.StopAnimMontage` null)
        (set `self.camMove` true)
        (set `self.bCanPlay` true)))))

(fn `UserConstructionScript`)